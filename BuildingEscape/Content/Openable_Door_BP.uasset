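; Openable door actor that swings open and closed by rotating the whole actor around yaw.
; It stores its initial rotation on BeginPlay, then responds to OnOpen and OnClose events from OpenDoor.
; Opening plays the DoorSwing timeline, whose OpenAngle track is scaled by DoorDirection and combined with the initial rotation.
; Closing reverses the same timeline.
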(event OnClose(OpenDoor)
  (bind _open_angle (Timeline|Door%20Swing Reverse)
    (:Update
      (Transformation|SetActorRotation (Math|Rotator|CombineRotators (Math|Rotator|MakeRotator 0.0 0.0 (* (Variables|Default|GetDoor%20Direction) _open_angle)) (Variables|Default|GetInitial%20Rotation))))))

(event OnOpen(OpenDoor)
  (bind _open_angle (Timeline|Door%20Swing Play)
    (:Update
      (Transformation|SetActorRotation (Math|Rotator|CombineRotators (Math|Rotator|MakeRotator 0.0 0.0 (* (Variables|Default|GetDoor%20Direction) _open_angle)) (Variables|Default|GetInitial%20Rotation))))))

(event EventBeginPlay
  (Variables|Default|SetInitial%20Rotation (Transformation|GetActorRotation)))

(fn ConstructionScript)